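; BP_DoorWayJumpScare is a jump scare actor that slides a mannequin to a set end point and then removes itself.
; Once the CalledJumScare flag is true, Tick moves the Mannequin toward EndPoint at constant Speed using VInterpToConstant, without sweeping for collision.
; The actor destroys itself when the mannequin reaches that point.
; Nothing in this Blueprint sets the trigger flag.
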(event EventTick
  (params (DeltaSeconds :type Float%20%28single-precision%29))
  (if (Variables|Default|GetbCalledJumScare)
    (Transformation|SetWorldLocation (Variables|Default|GetMannequin) (Math|Interpolation|VInterptoConstant (Transformation|GetWorldLocation (Variables|Default|GetMannequin)) (Transformation|GetWorldLocation (Variables|Default|GetEndPoint)) DeltaSeconds (Variables|Default|GetSpeed)) false false)
    (if (Math|Vector|Equal(Vector) (Transformation|GetWorldLocation (Variables|Default|GetMannequin)) (Transformation|GetWorldLocation (Variables|Default|GetEndPoint)) 0.0001)
      (Actor|DestroyActor))))

(fn ConstructionScript)