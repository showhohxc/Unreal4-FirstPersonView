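; Player controller that handles mouse look, the inventory menu toggle and the Return key.
; It creates a collapsed inventory widget at start and scales look input by a sensitivity value.
; When allowed, toggling shows or hides the menu while switching movement, look input and cursor.
; Opening also removes an on-screen exam widget, setting Game-and-UI input only in that case; Return fires PressedReturn.
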(event Custom|ToggleInventory
  (bind _w_examref (Variables|Default|GetW_ExamRef))
  (if (Variables|Default|GetbCanOpenInventory)
    (if (Variables|Default|GetIsInventoryOpen)
      (Variables|Default|SetIsInventoryOpen false)
      (Pawn|Components|CharacterMovement|SetMovementMode (Variables|/Script/Engine.Character|GetCharacterMovement (Game|GetPlayerCharacter 0)) "MOVE_Walking" 0)
      (Input|ResetIgnoreLookInput)
      (Variables|Default|SetbShowMouseCursor false)
      (Widget|SetVisibility (Variables|Default|GetW_InventoryMenuRef) "Collapsed")
      (Input|SetInputModeGameOnly self)
      (else
        (Variables|Default|SetIsInventoryOpen true)
        (Pawn|Components|CharacterMovement|DisableMovement (Variables|/Script/Engine.Character|GetCharacterMovement (Game|GetPlayerCharacter 0)))
        (Input|SetIgnoreLookInput true)
        (Variables|Default|SetbShowMouseCursor true)
        (Widget|SetVisibility (Variables|Default|GetW_InventoryMenuRef) "SelfHitTestInvisible")
        (if (UserInterface|Viewport|IsinViewport _w_examref)
          (Widget|RemovefromParent _w_examref)
          (Input|SetInputModeGameandUI self (Variables|Default|GetW_InventoryMenuRef) "DoNotLock" true))))))

(event EventBeginPlay
  (bind _returnvalue (UserInterface|CreateWidget "/Game/BluePrint/UMG/Inventory/W_Inventory_Menu.W_Inventory_Menu_C"))
  (bind _output_get (Variables|Default|SetW_InventoryMenuRef _returnvalue))
  (Widget|SetVisibility _output_get "Collapsed")
  (UserInterface|Viewport|AddtoViewport (Variables|Default|GetW_InventoryMenuRef) 0))

(event Input|ActionEvents|InputActionInventoryToggle
  (params (Key :type Key%20Structure :default "None"))
  (:Pressed
    (CallFunction|ToggleInventory)))

(event Input|ActionEvents|InputActionReturn
  (params (Key :type Key%20Structure :default "None"))
  (:Pressed
    (Default|CallPressedReturn)))

(event Input|AxisEvents|InputAxisLookUp
  (params (AxisValue :type Float%20%28single-precision%29))
  ;[1 1 1] Mouse Direction Control
  (Class|PlayerController|AddPitchInput (* AxisValue (Variables|Default|GetLookSensitivity))))

(event Input|AxisEvents|InputAxisLookRight
  (params (AxisValue :type Float%20%28single-precision%29))
  ;[1 1 1] Mouse Direction Control
  (Class|PlayerController|AddYawInput (* AxisValue (Variables|Default|GetLookSensitivity))))

(fn ConstructionScript)