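; Interactable hinged door that swings outward, choosing its yaw direction from which side the player or AI approaches, via a dot product.
; Interact toggles it on a timeline while CanInteract is true.
; AI_Classic entering the Box disables interaction and opens it on a second timeline; any overlap end reverses that timeline, restoring interaction when finished.
; Tick prints the dot product for debugging, and LockAfterActive only prints a message.
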(event OnComponentBeginOverlap(Box)
  (params (OverlappedComponent :type Primitive%20Component%20Object%20Reference) (OtherActor :type Actor%20Object%20Reference) (OtherComp :type Primitive%20Component%20Object%20Reference) (OtherBodyIndex :type Integer) (bFromSweep :type Boolean) (SweepResult :type Hit%20Result%20Structure%20%28by%20ref%29))
  (bind _self self)
  (bind _asai_classic (Utilities|Casting|CastToAI_Classic OtherActor))
  (Variables|Default|SetbCanInteract false)
  (if (Variables|Default|GetIsDoorClosed)
    (Variables|Default|SetIsDoorClosed false)
    (Variables|Default|SetDotProduct (Math|Vector|DotProduct (Math|Vector|Normalize (- (Transformation|GetActorLocation _self) (Transformation|GetActorLocation _asai_classic))) (Transformation|GetActorForwardVector _self)))
    (bind (_direction _alpha) (Timeline|OpenDoor_AI PlayFromStart)
      (:Update
        (Transformation|SetRelativeRotation (Variables|Default|GetStaticMesh1) (Math|Rotator|MakeRotator 0.0 0.0 (Math|Float|Lerp 0.0 (Math|Float|SelectFloat 9e+01 -9e+01 (>= (Variables|Default|GetDotProduct) 0.0)) _alpha)) false false))
      (:Finished
        (switch Utilities|FlowControl|Switch|SwitchonETimelineDirection _direction
          (:Backward
            (Variables|Default|SetbCanInteract true)))))))

(event OnComponentEndOverlap(Box)
  (params (OverlappedComponent :type Primitive%20Component%20Object%20Reference) (OtherActor :type Actor%20Object%20Reference) (OtherComp :type Primitive%20Component%20Object%20Reference) (OtherBodyIndex :type Integer))
  (if (not (Variables|Default|GetIsDoorClosed))
    (Variables|Default|SetIsDoorClosed true)
    (bind (_direction _alpha) (Timeline|OpenDoor_AI ReverseFromEnd)
      (:Update
        (Transformation|SetRelativeRotation (Variables|Default|GetStaticMesh1) (Math|Rotator|MakeRotator 0.0 0.0 (Math|Float|Lerp 0.0 (Math|Float|SelectFloat 9e+01 -9e+01 (>= (Variables|Default|GetDotProduct) 0.0)) _alpha)) false false))
      (:Finished
        (switch Utilities|FlowControl|Switch|SwitchonETimelineDirection _direction
          (:Backward
            (Variables|Default|SetbCanInteract true)))))))

(event EventBeginPlay
  (|CallParentFunction) ; 지금 이 노드는 비활성 상태입니다. \n핀을 끌어서 다른 노드를 연결하면 활성화됩니다.
)

(event Collision|EventActorBeginOverlap
  (params (OtherActor :type Actor%20Object%20Reference)))

(event EventLockAfterActive
  (Development|PrintString "BP_Interaction_OutWards Activate"))

(event EventInteract
  (bind _self self)
  (if (Variables|Default|GetbCanInteract)
    (if (Variables|Default|GetIsDoorClosed)
      (Variables|Default|SetIsDoorClosed false)
      (bind _output_get (Variables|Default|SetDotProduct (Math|Vector|DotProduct (Math|Vector|Normalize (- (Transformation|GetActorLocation _self) (Transformation|GetActorLocation (Variables|Default|GetPlayerRef)))) (Transformation|GetActorForwardVector _self))))
      (bind _alpha (Timeline|OpenDoorTimeLine PlayFromStart)
        (:Update
          (Transformation|SetRelativeRotation (Variables|Default|GetStaticMesh1) (Math|Rotator|MakeRotator 0.0 0.0 (Math|Float|Lerp 0.0 (Math|Float|SelectFloat 9e+01 -9e+01 (>= (Variables|Default|GetDotProduct) 0.0)) _alpha)) false false)))
      (else
        (Variables|Default|SetIsDoorClosed true)
        (Timeline|OpenDoorTimeLine ReverseFromEnd)))))

(event EventTick
  (params (DeltaSeconds :type Float%20%28single-precision%29))
  (Development|PrintString (Utilities|String|ToString(Float) (stale EventInteract _output_get)) true true "(R=0.000000,G=0.660000,B=1.000000,A=1.000000)" DeltaSeconds))

(fn ConstructionScript
  (|CallParentFunction))