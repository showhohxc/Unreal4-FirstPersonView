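; BP_Interaction_Door is an interactable door that swings open and closed when interacted with.
; Interact toggles IsDoorClosed and plays or reverses OpenDoorTimeLine, whose Alpha lerps StaticMesh1's relative yaw between closed and a quarter turn open.
; LockAfterActive only prints a debug string, and the construction script just calls its parent.
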(event EventBeginPlay
  (|CallParentFunction) ; 지금 이 노드는 비활성 상태입니다. \n핀을 끌어서 다른 노드를 연결하면 활성화됩니다.
)

(event Collision|EventActorBeginOverlap
  (params (OtherActor :type Actor%20Object%20Reference)))

(event EventTick
  (params (DeltaSeconds :type Float%20%28single-precision%29)))

(event EventInteract
  (if (Variables|Default|GetIsDoorClosed)
    (Variables|Default|SetIsDoorClosed false)
    (bind _alpha (Timeline|OpenDoorTimeLine Play)
      (:Update
        (Transformation|SetRelativeRotation (Variables|Default|GetStaticMesh1) (Math|Rotator|MakeRotator 0.0 0.0 (Math|Float|Lerp 0.0 -9e+01 _alpha)) false false)))
    (else
      (Variables|Default|SetIsDoorClosed true)
      (Timeline|OpenDoorTimeLine Reverse))))

(event EventLockAfterActive
  (Development|PrintString "BP_Interaction_Door"))

(fn ConstructionScript
  (|CallParentFunction))