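; Bandage inventory item, named as a variant of the Inventoryitem master, that restores player health when used.
; UseItem checks the player's BPCHealth component and, only if current health is below maximum, adds AmountHealthToAdd.
; It sets UseItemSucess to report whether the heal was applied.
; The BeginPlay, overlap and Tick events are disabled placeholders, and the construction script only calls the parent.
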(event EventBeginPlay
  (|CallParentFunction) ; 지금 이 노드는 비활성 상태입니다. \n핀을 끌어서 다른 노드를 연결하면 활성화됩니다.
)

(event Collision|EventActorBeginOverlap
  (params (OtherActor :type Actor%20Object%20Reference))
  (|CallParentFunction OtherActor) ; 지금 이 노드는 비활성 상태입니다. \n핀을 끌어서 다른 노드를 연결하면 활성화됩니다.
)

(event EventTick
  (params (DeltaSeconds :type Float%20%28single-precision%29))
  (|CallParentFunction DeltaSeconds) ; 지금 이 노드는 비활성 상태입니다. \n핀을 끌어서 다른 노드를 연결하면 활성화됩니다.
)

(event EventUseItem
  (bind _playerref (Variables|Default|GetPlayerRef))
  (bind _bpc_health (Variables|/Game/BluePrint/GameBP/Level_1/L1_Character.L1_Character_C|GetBPC_Health _playerref))
  (if (< (Variables|/Game/BluePrint/BluePrintComponent/BPC_Health.BPC_Health_C|GetCurrentHealth _bpc_health) (Variables|/Game/BluePrint/BluePrintComponent/BPC_Health.BPC_Health_C|GetMaxHealth _bpc_health))
    (Default|AddHealth _bpc_health (Variables|Default|GetAmountHealthToAdd))
    (Variables|Default|SetbUseItemSucess true)
    (else
      (Variables|Default|SetbUseItemSucess false))))

(fn ConstructionScript
  (|CallParentFunction))