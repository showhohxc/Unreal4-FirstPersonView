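; Backpack pickup actor that adds extra slots to the player's inventory component, then destroys itself when Action is pressed.
; Sphere overlap with an L1_Character starts per-tick checks and shows a prompt widget kept above the mesh.
; While active, a visibility trace to the player camera hides the prompt if blocked, otherwise turns it toward the camera.
; Trace length against PickupDistance toggles the prompt state and the actor's input.
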(event OnComponentBeginOverlap(Sphere)
  (params (OverlappedComponent :type Primitive%20Component%20Object%20Reference) (OtherActor :type Actor%20Object%20Reference) (OtherComp :type Primitive%20Component%20Object%20Reference) (OtherBodyIndex :type Integer) (bFromSweep :type Boolean) (SweepResult :type Hit%20Result%20Structure%20%28by%20ref%29))
  (bind _asl1_character (Utilities|Casting|CastToL1_Character OtherActor))
  (Variables|Default|SetPlayer_Ref _asl1_character)
  (Rendering|SetVisibility (Variables|Default|GetPickupWidget) true false)
  (Variables|Default|SetbUpdateActor true))

(event OnComponentEndOverlap(Sphere)
  (params (OverlappedComponent :type Primitive%20Component%20Object%20Reference) (OtherActor :type Actor%20Object%20Reference) (OtherComp :type Primitive%20Component%20Object%20Reference) (OtherBodyIndex :type Integer))
  (Utilities|Casting|CastToL1_Character OtherActor)
  (Rendering|SetVisibility (Variables|Default|GetPickupWidget) false false)
  (Variables|Default|SetbUpdateActor false)
  (Input|DisableInput (Game|GetPlayerController 0)))

(event EventBeginPlay)

(event Collision|EventActorBeginOverlap
  (params (OtherActor :type Actor%20Object%20Reference)))

(event EventTick
  (params (DeltaSeconds :type Float%20%28single-precision%29))
  (bind _returnvalue (Game|GetPlayerController 0))
  (bind _pickupwidget (Variables|Default|GetPickupWidget))
  (bind _backpackmesh (Variables|Default|GetBackpackMesh))
  (bind _returnvalue_2 (Transformation|GetWorldLocation _backpackmesh))
  (Transformation|SetWorldLocation (Variables|Default|GetPickupWidget) (Math|Vector|MakeVector (.x _returnvalue_2) (.y _returnvalue_2) (+ (.z _returnvalue_2) (Variables|Default|GetWidgetDistanceAboveMesh))) false false)
  (if (Variables|Default|GetbUpdateActor)
    (bind (_outhit _returnvalue_3) (Collision|LineTraceByChannel (Transformation|GetActorLocation) (Transformation|GetWorldLocation (Variables|/Game/BluePrint/GameBP/Level_1/L1_Character.L1_Character_C|GetCamera (Variables|Default|GetPlayer_Ref))) "TraceTypeQuery1" false 0 "ForDuration"))
    (if (not _returnvalue_3)
      (Rendering|SetVisibility _pickupwidget true false)
      (Transformation|SetWorldRotation (Variables|Default|GetPickupWidget) (Math|Rotator|FindLookatRotation (Transformation|GetWorldLocation (Variables|Default|GetPickupWidget)) (Transformation|GetWorldLocation (Variables|/Game/BluePrint/GameBP/Level_1/L1_Character.L1_Character_C|GetCamera (Variables|Default|GetPlayer_Ref)))) false false)
      (Default|TogglePrompt (.AsW%20Pickup%20Prompt (Utilities|Casting|CastToW_PickupPrompt (UserInterface|GetUserWidgetObject (Variables|Default|GetPickupWidget)))) (<= (Math|Vector|VectorLength (- (.TraceStart (Collision|BreakHitResult _outhit)) (.TraceEnd (Collision|BreakHitResult _outhit)))) (Variables|Default|GetPickupDistance)))
      (if (<= (Math|Vector|VectorLength (- (.TraceStart (Collision|BreakHitResult _outhit)) (.TraceEnd (Collision|BreakHitResult _outhit)))) (Variables|Default|GetPickupDistance))
        (Input|EnableInput _returnvalue)
        (else
          (Input|DisableInput _returnvalue)))
      (else
        (Rendering|SetVisibility _pickupwidget false false)
        (Input|DisableInput (Game|GetPlayerController 0))))))

(event Input|ActionEvents|InputActionAction
  (params (Key :type Key%20Structure :default "None"))
  (:Pressed
    (Default|AddMoreSlots (Variables|/Game/BluePrint/GameBP/Level_1/L1_Character.L1_Character_C|GetBPC_Inventory (Variables|Default|GetPlayer_Ref)) (Variables|Default|GetAmountofSlots))
    (Actor|DestroyActor)))

(fn ConstructionScript)