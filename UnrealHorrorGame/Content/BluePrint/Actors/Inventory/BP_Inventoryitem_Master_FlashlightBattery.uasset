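; Flashlight battery inventory item, apparently a child of the inventory item master, that recharges the player's flashlight when used.
; UseItem adds BatteryAmount through the player's BPCFlashlight component only while its charge is below maximum, setting UseItemSucess to report the result.
; On success it also sends the "UserBattery" objective completion to the GameState without immediately setting the next objective, and plays the quest success sound.
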(event EventBeginPlay
  (|CallParentFunction) ; 지금 이 노드는 비활성 상태입니다. \n핀을 끌어서 다른 노드를 연결하면 활성화됩니다.
)

(event Collision|EventActorBeginOverlap
  (params (OtherActor :type Actor%20Object%20Reference))
  (|CallParentFunction OtherActor) ; 지금 이 노드는 비활성 상태입니다. \n핀을 끌어서 다른 노드를 연결하면 활성화됩니다.
)

(event EventTick
  (params (DeltaSeconds :type Float%20%28single-precision%29))
  (|CallParentFunction DeltaSeconds) ; 지금 이 노드는 비활성 상태입니다. \n핀을 끌어서 다른 노드를 연결하면 활성화됩니다.
)

(event EventUseItem
  (bind _playerref (Variables|Default|GetPlayerRef))
  (bind _bpc_flashlight (Variables|/Game/BluePrint/GameBP/Level_1/L1_Character.L1_Character_C|GetBPC_Flashlight _playerref))
  (if (< (Variables|/Game/BluePrint/BluePrintComponent/BPC_Flashlight.BPC_Flashlight_C|GetCurrentBatteryLevel _bpc_flashlight) (Variables|/Game/BluePrint/BluePrintComponent/BPC_Flashlight.BPC_Flashlight_C|GetMaxBatteryLevel _bpc_flashlight))
    (Default|AddBatteryLife _bpc_flashlight (Variables|Default|GetBatteryAmount))
    (Variables|Default|SetbUseItemSucess true)
    (Class|BPIObjectiveCall|CompleteObjectiveCall(Message) (Game|GetGameState) "UserBattery" false)
    (Audio|PlaySound2D "/Game/BluePrint/Sounds/QuestSucess.QuestSucess" 1.0 1.0 0.0 0 0)
    (else
      (Variables|Default|SetbUseItemSucess false))))

(fn ConstructionScript
  (|CallParentFunction))