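; Locker hiding spot, a hide actor child that adds a swinging door to the parent's interaction.
; Interact locks re-entry, swings the door open on a timeline, then calls the parent Interact after a short delay.
; When the parent's move-finished event fires, the door closes after a pause and re-enables interaction.
; EnemyFind disables interaction and door collision, then swings the door open without closing it.
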(event Custom|CloseDoor
  (bind _alpha (Timeline|타임라인_0 Play)
    (:Update
      (Transformation|SetRelativeRotation (Variables|Default|GetStaticMesh1) (Math|Rotator|MakeRotator 0.0 0.0 (Math|Float|Lerp 9e+01 0.0 _alpha)) false false))
    (:Finished
      (Variables|Default|SetbCanInteract true))))

(event Custom|FinishedMoveingEnd_Event
  (Utilities|FlowControl|Delay 0.2)
  (CallFunction|CloseDoor))

(event EventBeginPlay
  (|CallParentFunction)
  (EventDispatchers|AssignFinishedMoveingEnd (delegate Custom|FinishedMoveingEnd_Event)))

(event EventEnemyFind
  (Variables|Default|SetbCanInteract false)
  (Collision|SetCollisionEnabled (Variables|Default|GetStaticMesh1) "NoCollision")
  (bind _alpha (Timeline|AIOpenDoor PlayFromStart)
    (:Update
      (Transformation|SetRelativeRotation (Variables|Default|GetStaticMesh1) (Math|Rotator|MakeRotator 0.0 0.0 (Math|Float|Lerp 0.0 9e+01 _alpha)) false false))
    (:Finished
      (Utilities|FlowControl|Delay 0.2))))

(event EventInteract
  (if (Variables|Default|GetbCanInteract)
    (Variables|Default|SetbCanInteract false)
    (bind _alpha (Timeline|OpenLockerDoorTimeline Play)
      (:Update
        (Transformation|SetRelativeRotation (Variables|Default|GetStaticMesh1) (Math|Rotator|MakeRotator 0.0 0.0 (Math|Float|Lerp 0.0 9e+01 _alpha)) false false))
      (:Finished
        (Utilities|FlowControl|Delay 0.2)
        (|CallParentFunction)))))

(fn ConstructionScript
  (|CallParentFunction))