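; BP_CameraController is an interactable actor that lets the player view the level's security cameras.
; At BeginPlay it caches the player character, controller and every BP_SecurityCamera.
; Interact toggles viewing, transferring input from the character to this actor, hiding the HUD and switching the view target.
; CameraLeft/Right cycle with wraparound, while Return or Action restores the player's view, input and HUD and resets the index.
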(event Custom|LeaveCameraController
  (bind _playercontrollerref (Variables|Default|GetPlayerControllerRef))
  (Variables|Default|SetIsViewingCameras false)
  (Input|DisableInput _playercontrollerref)
  (Input|ResetIgnoreLookInput _playercontrollerref)
  (Widget|SetVisibility (Variables|/Game/BluePrint/GameBP/Level_1/L1_Character.L1_Character_C|GetMainHUD (Variables|Default|GetPlayerCharRef)) "Visible")
  (Input|EnableInput (Variables|Default|GetPlayerCharRef) (Variables|Default|GetPlayerControllerRef))
  (Variables|Default|SetCurrentCameraIndex 0)
  (Game|Player|SetViewTargetwithBlend (Variables|Default|GetPlayerControllerRef) (Variables|Default|GetPlayerCharRef) 0.0 "VTBlend_Linear" 0.0 false)
  (Development|PrintString "DeActivate"))

(event EventBeginPlay
  (bind _asl1_character (Utilities|Casting|CastToL1_Character (Game|GetPlayerCharacter 0)))
  (Variables|Default|SetPlayerCharRef _asl1_character)
  (bind _ashg_player_controller (Utilities|Casting|CastToHG_PlayerController (Game|GetPlayerController 0)))
  (Variables|Default|SetPlayerControllerRef _ashg_player_controller)
  (bind _outactors (Actor|GetAllActorsOfClass "/Game/BluePrint/Actors/SecurityCameras/BP_SecurityCamera.BP_SecurityCamera_C"))
  (Variables|Default|SetSecurityCameras _outactors))

(event Collision|EventActorBeginOverlap
  (params (OtherActor :type Actor%20Object%20Reference)))

(event EventTick
  (params (DeltaSeconds :type Float%20%28single-precision%29)))

(event EventInteract
  (bind _playercontrollerref (Variables|Default|GetPlayerControllerRef))
  (if (Variables|Default|GetIsViewingCameras)
    (CallFunction|LeaveCameraController)
    (else
      (Variables|Default|SetIsViewingCameras true)
      (Input|DisableInput (Variables|Default|GetPlayerCharRef) _playercontrollerref)
      (Input|SetIgnoreLookInput _playercontrollerref true)
      (Widget|SetVisibility (Variables|/Game/BluePrint/GameBP/Level_1/L1_Character.L1_Character_C|GetMainHUD (Variables|Default|GetPlayerCharRef)) "Hidden")
      (Input|EnableInput (Variables|Default|GetPlayerControllerRef))
      (CallFunction|ViewThroughCamera)
      (Development|PrintString "Activate"))))

(event Input|ActionEvents|InputActionCameraRight
  (params (Key :type Key%20Structure :default "None"))
  (:Pressed
    (Variables|Default|SetCurrentCameraIndex (select (> (+ (Variables|Default|GetCurrentCameraIndex) 1) (- (Utilities|Array|Length (Variables|Default|GetSecurityCameras)) 1)) 0 (+ (Variables|Default|GetCurrentCameraIndex) 1)))
    (CallFunction|ViewThroughCamera)))

(event Input|ActionEvents|InputActionCameraLeft
  (params (Key :type Key%20Structure :default "None"))
  (:Pressed
    (Variables|Default|SetCurrentCameraIndex (select (>= (+ (Variables|Default|GetCurrentCameraIndex) -1) 0) (+ (Variables|Default|GetCurrentCameraIndex) -1) (- (Utilities|Array|Length (Variables|Default|GetSecurityCameras)) 1)))
    (CallFunction|ViewThroughCamera)))

(event Input|ActionEvents|InputActionAction
  (params (Key :type Key%20Structure :default "None"))
  (:Pressed
    (CallFunction|LeaveCameraController)))

(event Input|ActionEvents|InputActionReturn
  (params (Key :type Key%20Structure :default "None"))
  (:Pressed
    (CallFunction|LeaveCameraController)))

(fn ConstructionScript)

(fn ViewThroughCamera
  (Game|Player|SetViewTargetwithBlend (Variables|Default|GetPlayerControllerRef) (Utilities|Array|Get(acopy) (Variables|Default|GetSecurityCameras) (Variables|Default|GetCurrentCameraIndex)) 0.0 "VTBlend_Linear" 0.0 false)
  (return))